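; Player controller for multiplayer that requests player spawns and manages a world-space crosshair for the local player.
; On BeginPlay the local controller calls ROS_SpawnPlayer, which on authority asks GM_Multiplayer to spawn the player, then spawns a crosshair actor.
; SetCrosshairLocation moves that actor to the hit location or, without a hit, the trace end.
; PlayerDeath calls the same spawn event again after a delay.
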(event Custom|SetCrosshairLocation
  (params (Hit :type Boolean) (Hit%20Location :type Vector) (Trace%20End :type Vector))
  (if (Pawn|IsLocalPlayerController)
    (bind _crosshairwidget (Variables|Default|GetCrosshairWidget)
      (:then
        (if Hit
          (Transformation|SetActorLocation _crosshairwidget Hit%20Location false false)
          (else
            (Transformation|SetActorLocation _crosshairwidget Trace%20End false false))))
      (:else))))

(event Custom|ROS_SpawnPlayer
  (Networking|SwitchHasAuthority
    (:Authority
      (bind _asgm_multiplayer (Utilities|Casting|CastToGM_Multiplayer (Game|GetGameMode)))
      (Default|SpawnPlayer _asgm_multiplayer self))))

(event Custom|PlayerDeath
  (Utilities|FlowControl|Delay 1e+01)
  (CallFunction|ROSSpawnPlayer))

(event EventBeginPlay
  (if (Pawn|IsLocalPlayerController)
    (CallFunction|ROSSpawnPlayer)
    (bind _returnvalue (Game|SpawnActorfromClass "/Game/Multiplayer/UI/BP_CrossHairWidget.BP_CrossHairWidget_C" (Math|Transform|MakeTransform "0, 0, 0" "0, 0, 0" "1.000000,1.000000,1.000000") "Undefined" "MultiplyWithRoot" 0 0))
    (Variables|Default|SetCrosshairWidget _returnvalue)))

(fn ConstructionScript)