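; Multiplayer game mode Blueprint that spawns or respawns a player's third-person character at a random Player Start.
; SpawnPlayer destroys the controller's current pawn if one exists, spawns a new character and has the controller possess it.
; FindRandomPlayerStart supplies the spawn location and rotation by picking randomly among all PlayerStart actors, with no occupancy check.
; The event graph and construction script hold no logic, and nothing in this file calls SpawnPlayer.
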(event EventBeginPlay)

(event EventTick
  (params (DeltaSeconds :type Float%20%28single-precision%29)))

(fn ConstructionScript)

(fn FindRandomPlayerStart
  (bind _outactors (Actor|GetAllActorsOfClass "/Script/Engine.PlayerStart"))
  (return (Transformation|GetActorTransform (Utilities|Array|Get(acopy) _outactors (Math|Random|RandomIntegerinRange 0 (- (Utilities|Array|Length _outactors) 1))))))

(fn SpawnPlayer
  (params (Player%20Controller :type Player%20Controller%20Object%20Reference))
  (bind _returnvalue (Pawn|GetControlledPawn Player%20Controller))
  (bind _player_start_transform (CallFunction|FindRandomPlayerStart))
  (Utilities|IsValid _returnvalue
    (:Is%20Valid
      (Actor|DestroyActor _returnvalue))
    (:Is%20Not%20Valid
      _))
  (bind _returnvalue_2 (Game|SpawnActorfromClass "/Game/Multiplayer/Blueprints/BP_ThirdPersonCharacterTPS.BP_ThirdPersonCharacterTPS_C" (Math|Transform|MakeTransform (.location _player_start_transform) (.rotation _player_start_transform) "1.000000,1.000000,1.000000") "Undefined" "MultiplyWithRoot" 0 0))
  (Pawn|Possess Player%20Controller _returnvalue_2))